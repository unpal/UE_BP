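; BP_Startup2 is an actor Blueprint that continuously spins itself and its SMCube1 component.
; Each Tick adds a fixed yaw step to the cube's relative rotation, then a smaller one to the whole actor, zeroing pitch and roll on both.
; The steps ignore delta time, so spin speed depends on frame rate.
; An unconnected node that would nudge the actor along X never runs.
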(event EventTick
  (params (DeltaSeconds :type Float%20%28single-precision%29))
  (bind _sm_cube1 (Variables|Default|GetSM_Cube1))
  (Utilities|FlowControl|Sequence
    (:then_0
      (Transformation|SetRelativeRotation _sm_cube1 (Math|Rotator|MakeRotator 0.0 0.0 (+ (.yaw (Variables|/Script/Engine.SceneComponent|GetRelativeRotation _sm_cube1)) 2.0)) false false))
    (:then_1
      (Transformation|SetActorRotation (Math|Rotator|MakeRotator 0.0 0.0 (+ (.yaw (Transformation|GetActorRotation)) 1.0))))))

(fn ConstructionScript)